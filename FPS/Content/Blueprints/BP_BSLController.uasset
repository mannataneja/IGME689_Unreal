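; BP_BSLController is a debug controller actor that inspects the sublayer tree of an ArcGIS Building Scene Layer.
; On BeginPlay it fetches the map from the ArcGISMapActor and takes the layer at index 1.
; ParseBSL then descends fixed sublayer indices with delays, prints a name and decrements Position, with no loop.
; The visibility toggle is disconnected, and the ParseSublayer helper, which prints the first sublayer's name, is not called here.
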(event Custom|ParseBSL
  (bind _returnvalue (Utilities|String|ToString(Integer) 1))
  (bind _asarc_gisbuilding_scene_layer (Utilities|Casting|CastToArcGISBuildingSceneLayer (Variables|Default|GetBuildingSceneLayer))
    (:then
      (Utilities|IsValid _asarc_gisbuilding_scene_layer
        (:Is%20Valid
          (bind _returnvalue_2 (Class|ArcGISBuildingSceneLayer|GetSublayers _asarc_gisbuilding_scene_layer))
          (Utilities|FlowControl|Delay 1.0)
          (bind _returnvalue_3 (Class|ArcGISBuildingSceneSublayer|GetSublayers (Class|ArcGISBuildingSceneSublayerImmutableCollection|At _returnvalue_2)))
          (Utilities|FlowControl|Delay 0.5)
          (bind _returnvalue_4 (Class|ArcGISBuildingSceneSublayer|GetSublayers (Class|ArcGISBuildingSceneSublayerImmutableCollection|At _returnvalue_3 2)))
          (bind _returnvalue_5 (Class|ArcGISBuildingSceneSublayerImmutableCollection|GetSize _returnvalue_4))
          (Development|PrintString _returnvalue)
          (if (< 0 _returnvalue_5)
            (Utilities|FlowControl|Delay 0.2)
            (bind _returnvalue_6 (Class|ArcGISBuildingSceneSublayer|GetName (Class|ArcGISBuildingSceneSublayerImmutableCollection|At _returnvalue_4 (Class|KismetStringLibrary|ToInt64(String) _returnvalue))))
            (Development|PrintString _returnvalue_6)
            (Variables|Default|SetPosition (+ (Variables|Default|GetPosition) -1))
            (else
              (Utilities|Time|ClearandInvalidateTimerbyHandle (Variables|Default|GetTimerHandle)))))))
    (:CastFailed
      (Development|PrintString "Cast to BSL Failed"))))

(event EventBeginPlay
  (bind _returnvalue (Actor|GetActorOfClass "/Script/ArcGISMapsSDK.ArcGISMapActor"))
  (bind _output_get (Variables|Default|SetMapComponent _returnvalue))
  (bind _returnvalue_2 (Class|ArcGISMapComponent|GetMap (Variables|/Script/ArcGISMapsSDK.ArcGISMapActor|GetMapComponent _output_get)))
  (bind _returnvalue_3 (Class|ArcGISMap|GetLayers _returnvalue_2))
  (bind _returnvalue_4 (Class|ArcGISLayerCollection|GetSize _returnvalue_3))
  (if (!= _returnvalue_4 0)
    (bind _output_get_2 (Variables|Default|SetBuildingSceneLayer (Class|ArcGISLayerCollection|At _returnvalue_3 1)))
    (bind _returnvalue_5 (Class|ArcGISLayer|GetName _output_get_2))
    (Development|PrintString _returnvalue_5)
    (Utilities|FlowControl|Delay 0.5)
    (CallFunction|ParseBSL)))

(event Collision|EventActorBeginOverlap
  (params (OtherActor :type Actor%20Object%20Reference)))

(event EventTick
  (params (DeltaSeconds :type Float%20%28single-precision%29)))

(fn ConstructionScript)

(fn ParseSublayer
  (bind _asarc_gisbuilding_scene_layer (Utilities|Casting|CastToArcGISBuildingSceneLayer (Variables|Default|GetBuildingSceneLayer))
    (:then
      (Utilities|IsValid _asarc_gisbuilding_scene_layer
        (:Is%20Valid
          (bind _returnvalue (Class|ArcGISBuildingSceneLayer|GetSublayers _asarc_gisbuilding_scene_layer))
          (bind _returnvalue_2 (Class|ArcGISBuildingSceneSublayerImmutableCollection|GetSize _returnvalue))
          (bind _returnvalue_3 (Class|ArcGISBuildingSceneSublayer|GetName (Class|ArcGISBuildingSceneSublayerImmutableCollection|At _returnvalue)))
          (Development|PrintString _returnvalue_3))))
    (:CastFailed
      (Development|PrintString "Cast to BSL Failed"))))