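; Player-driven car with a countdown timer that ends in a win or lose screen.
; Throttle and Steer axes ease speed and steering with FInterpTo, and Tick offsets the actor without sweep, scaling yaw by speed.
; While Start is set, a Delay inside Tick paces the countdown.
; At minute rollover it shows the win widget if Win is set, or lose if time is out, and removes the timer widget.
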(event EventBeginPlay)

(event EventTick
  (params (DeltaSeconds :type Float%20%28single-precision%29))
  (bind _currentspeed (Variables|Default|GetCurrentSpeed))
  (Transformation|AddActorWorldOffset (* (* (Transformation|GetActorForwardVector) _currentspeed) DeltaSeconds))
  (Class|Actor|AddActorWorldRotation (Math|Rotator|MakeRotator 0.0 0.0 (* _currentspeed (Variables|Default|GetCurrentSteeringAngle) (Variables|Default|GetSpeedToRotationFactor) (Utilities|Time|GetWorldDeltaSeconds))))
  (if (Variables|Default|Getstart)
    (Utilities|FlowControl|Delay 1.0)
    (Variables|Default|SetSeconds (- (Variables|Default|GetSeconds) 1))
    (if (< (Variables|Default|GetSeconds) 0)
      (Variables|Default|SetMinutes (- (Variables|Default|GetMinutes) 1))
      (Variables|Default|SetSeconds 59)
      (if (Variables|Default|Getwin)
        (bind _returnvalue (UserInterface|CreateWidget "/Game/Blueprints/wbp_win.wbp_win_C"))
        (UserInterface|Viewport|AddtoViewport _returnvalue 0)
        (bind _foundwidgets (Widget|GetAllWidgetsOfClass "/Game/Blueprints/wbp_timer.wbp_timer_C" true))
        (Widget|RemovefromParent _foundwidgets)
        (elif (and (< (Variables|Default|GetMinutes) 0) (not (Variables|Default|Getwin)))
          (bind _returnvalue_2 (UserInterface|CreateWidget "/Game/Blueprints/wbp_lose.wbp_lose_C"))
          (UserInterface|Viewport|AddtoViewport _returnvalue_2 0)
          (bind _foundwidgets_2 (Widget|GetAllWidgetsOfClass "/Game/Blueprints/wbp_timer.wbp_timer_C" true))
          (Widget|RemovefromParent _foundwidgets_2))))))

(event Input|AxisEvents|InputAxisThrottle
  (params (AxisValue :type Float%20%28single-precision%29))
  (Variables|Default|SetCurrentSpeed (Math|Interpolation|FInterpTo (Variables|Default|GetCurrentSpeed) (* AxisValue (Variables|Default|GetMaxSpeed)) (Utilities|Time|GetWorldDeltaSeconds) 4.0)))

(event Input|AxisEvents|InputAxisSteer
  (params (AxisValue :type Float%20%28single-precision%29))
  (Variables|Default|SetCurrentSteeringAngle (Math|Interpolation|FInterpTo (Variables|Default|GetCurrentSteeringAngle) (* AxisValue (Variables|Default|GetMaxSteeringAngle)) (Utilities|Time|GetWorldDeltaSeconds) 4.0)))

(fn ConstructionScript)