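; Actor Blueprint that builds a spline from geographic coordinates on an ArcGIS map.
; On BeginPlay it caches the level's ArcGISMapActor.
; PopulateSpline turns each longitude and latitude into a zero-altitude ArcGIS point, converts it to engine position through the map component and appends it to the spline, printing a debug string.
; Despite the name, it creates no spline meshes, and an AddSplinePoint node is left unconnected.
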(event EventBeginPlay
  (bind _returnvalue (Actor|GetActorOfClass "/Script/ArcGISMapsSDK.ArcGISMapActor"))
  (Variables|Default|SetMapComponent _returnvalue))

(fn ConstructionScript)

(fn PopulateSpline
  (params (Longitude :type Float%20%28double-precision%29) (Latitude :type Float%20%28double-precision%29))
  (bind _returnvalue (Class|ArcGISPoint|CreateArcGISPointwithXYZ Longitude Latitude 0.0))
  (bind _returnvalue_2 (Class|ArcGISMapComponent|TransformPointtoEnginePosition (Variables|/Script/ArcGISMapsSDK.ArcGISMapActor|GetMapComponent (Variables|Default|GetMapComponent)) _returnvalue))
  (Class|SplineComponent|AddPoint (Variables|Default|GetSpline) (Utilities|Struct|MakeSplinePoint 0.0 _returnvalue_2 "0.000000,0.000000,0.000000" "0.000000,0.000000,0.000000" "0.000000,0.000000,0.000000" "1.000000,1.000000,1.000000" "Curve") true)
  (Development|PrintString "spline point"))