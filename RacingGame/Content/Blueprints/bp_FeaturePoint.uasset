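; Geographic feature point actor for an ArcGIS map that anchors checkpoints for a car.
; SpawnFeaturePoint places it on the ground at a WGS84 longitude and latitude.
; UpdatePosition moves the ArcGIS pawn above given coordinates and recenters the map origin there, using references cached on BeginPlay.
; SpawnCheckpoint spawns an actor at the point and moves Bp_car there with fixed rotation, while SpawnCheckPointHalfway spawns a halfway checkpoint.
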(event EventBeginPlay
  (bind _returnvalue (Actor|GetActorOfClass "/Script/ArcGISMapsSDK.ArcGISMapActor"))
  (Variables|Default|SetMapComponent _returnvalue)
  (bind _returnvalue_2 (Actor|GetActorOfClass "/Script/ArcGISSamples.ArcGISPawn"))
  (Variables|Default|SetPawn _returnvalue_2))

(event Collision|EventActorBeginOverlap
  (params (OtherActor :type Actor%20Object%20Reference)))

(event EventTick
  (params (DeltaSeconds :type Float%20%28single-precision%29)))

(fn ConstructionScript)

(fn UpdatePosition
  (params (Longitude :type Float%20%28double-precision%29) (Latitude :type Float%20%28double-precision%29))
  (bind _returnvalue (Class|ArcGISSpatialReference|WGS84))
  (bind _returnvalue_2 (Class|ArcGISPoint|CreateArcGISPointwithXYZSpatialReference Longitude Latitude 3e+03 _returnvalue))
  (Class|ArcGISLocationComponent|SetPosition (Actor|GetComponentbyClass (Variables|Default|GetPawn) "/Script/ArcGISMapsSDK.ArcGISLocationComponent") _returnvalue_2)
  (bind _returnvalue_3 (Class|ArcGISPoint|CreateArcGISPointwithXYZSpatialReference Longitude Latitude 0.0 _returnvalue))
  (Class|ArcGISMapComponent|SetOriginPosition (Variables|/Script/ArcGISMapsSDK.ArcGISMapActor|GetMapComponent (Variables|Default|GetMapComponent)) _returnvalue_3)
  (bind _returnvalue_4 (Actor|GetActorOfClass "/Script/ArcGISMapsSDK.ArcGISMapActor"))
  (Class|ArcGISMapComponent|SetOriginPosition (Variables|/Script/ArcGISMapsSDK.ArcGISMapActor|GetMapComponent _returnvalue_4) _returnvalue_3))

(fn SpawnFeaturePoint
  (params (Longitude :type Float%20%28double-precision%29) (Latitude :type Float%20%28double-precision%29))
  (bind _arcgislocation (Variables|Default|GetArcGISLocation))
  (bind _returnvalue (Class|ArcGISSpatialReference|WGS84))
  (bind _returnvalue_2 (Class|ArcGISPoint|CreateArcGISPointwithXYZSpatialReference Longitude Latitude 0.0 _returnvalue))
  (Class|ArcGISLocationComponent|SetPosition _arcgislocation _returnvalue_2)
  (Class|ArcGISLocationComponent|SetSurfacePlacementMode _arcgislocation "OnTheGround"))

(fn SpawnCheckpoint
  (bind _defaultsceneroot (Variables|Default|GetDefaultSceneRoot))
  (bind _returnvalue (Transformation|GetWorldLocation _defaultsceneroot))
  (bind _returnvalue_2 (Math|Conversions|ToTransform(Vector) _returnvalue))
  (Game|SpawnActorfromClass "/Game/Blueprints/bp_checkpoint.bp_checkpoint_C" _returnvalue_2 "Undefined" "MultiplyWithRoot" 0 0)
  (bind _returnvalue_3 (Actor|GetActorOfClass "/Game/Blueprints/bp_car.bp_car_C"))
  (Transformation|SetWorldTransform (Variables|/Game/Blueprints/bp_car.bp_car_C|GetDefaultSceneRoot _returnvalue_3) _returnvalue_2 false false)
  (Transformation|SetWorldRotation (Variables|/Game/Blueprints/bp_car.bp_car_C|GetDefaultSceneRoot _returnvalue_3) "0.000000,-90.000000,0.000000" false false))

(fn SpawnCheckPointHalfway
  (Game|SpawnActorfromClass "/Game/Blueprints/bp_checkpoint_halfway.bp_checkpoint_halfway_C" (Math|Conversions|ToTransform(Vector) (Transformation|GetWorldLocation (Variables|Default|GetDefaultSceneRoot))) "Undefined" "MultiplyWithRoot" 0 0))